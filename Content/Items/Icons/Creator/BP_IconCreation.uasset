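; BP_IconCreation is an icon-creation rig that frames a static or skeletal mesh for a SceneCapture2D.
; Each event assigns the mesh, sizes the ortho width from its bounding sphere and makes it the show-only component.
; Static meshes are framed by moving the capture along X from the bounds, while skeletal meshes move to a fixed offset.
; The construction script defaults the show-only component to the skeletal mesh.
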(event Custom|SkeletalMeshIcon
  (params (StaticMesh :type Skeletal%20Mesh%20Object%20Reference))
  (Components|SkeletalMesh|SetSkeletalMeshAsset (Variables|Default|GetSkeletalMesh) StaticMesh)
  (Variables|/Script/Engine.SceneCaptureComponent2D|SetOrthoWidth (Variables|Default|GetSceneCaptureComponent2D) (* (.sphereradius (StaticMesh|GetBounds StaticMesh)) 2.1))
  (Transformation|SetRelativeLocation (Variables|Default|GetSkeletalMesh) "50.000000,28.000000,-10.000000" false false)
  (Rendering|SceneCapture|ShowOnlyComponent (Variables|Default|GetSceneCaptureComponent2D) (Variables|Default|GetSkeletalMesh)))

(event Custom|StaticMeshIcon
  (params (StaticMesh :type Static%20Mesh%20Object%20Reference))
  (bind _returnvalue (StaticMesh|GetBounds StaticMesh))
  (Components|StaticMesh|SetStaticMesh (Variables|Default|GetStaticMesh) StaticMesh)
  (Variables|/Script/Engine.SceneCaptureComponent2D|SetOrthoWidth (Variables|Default|GetSceneCaptureComponent2D) (* (.sphereradius _returnvalue) 2.1))
  (Transformation|SetRelativeLocation (Variables|Default|GetSceneCaptureComponent2D) (+ (.origin _returnvalue) (Math|Vector|MakeVector (* (.x (.boxextent _returnvalue)) 3.0) 0.0 0.0)) false false)
  (Rendering|SceneCapture|ShowOnlyComponent (Variables|Default|GetSceneCaptureComponent2D) (Variables|Default|GetStaticMesh)))

(fn ConstructionScript
  (Rendering|SceneCapture|ShowOnlyComponent (Variables|Default|GetSceneCaptureComponent2D) (Variables|Default|GetSkeletalMesh)))